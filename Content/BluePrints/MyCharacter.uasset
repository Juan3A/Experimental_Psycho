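; Player character Blueprint that manages health, medkits and ammunition through keyboard and mouse input.
; Tab heals with a medkit up to a health cap, R refills the magazine from reserve ammo, and left click only decrements magazine ammo.
; Tick polls health through Dead, which pauses the game, shows a GameOver widget and enables the cursor at zero.
; O clears ManagerSound and plays a 2D fire sound.
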(event EventBeginPlay)

(event Collision|EventActorBeginOverlap
  (params (OtherActor :type Actor%20Object%20Reference)))

(event EventTick
  (params (DeltaSeconds :type Float%20%28single-precision%29))
  (CallFunction|Dead))

(event Input|MouseEvents|LeftMouseButton
  (params (Key :type Key%20Structure))
  (:Pressed
    (CallFunction|Shoot)))

(event Input|KeyboardEvents|O
  (params (Key :type Key%20Structure))
  (:Pressed
    (Variables|Default|SetManager%20Sound 0)
    (Audio|PlaySound2D "/Game/StarterContent/Audio/Fire01.Fire01" 1.0 1.0 0.0 0 0)))

(event Input|KeyboardEvents|R
  (params (Key :type Key%20Structure))
  (:Pressed
    (CallFunction|RecargarArma)))

(event Input|KeyboardEvents|Tab
  (params (Key :type Key%20Structure))
  (:Pressed
    (CallFunction|Curarse)))

(fn ConstructionScript)

(fn Dead
  (if (<= (Variables|Default|Gethp) 0.0)
    (Game|SetGamePaused true)
    (bind _returnvalue (UserInterface|CreateWidget "/Game/UI/GameOver.GameOver_C"))
    (UserInterface|Viewport|AddtoViewport _returnvalue 0)
    (Variables|/Script/Engine.PlayerController|SetbShowMouseCursor (Game|GetPlayerController 0) true)))

(fn Curarse
  (if (> (Variables|Default|GetBotiquin) 0)
    (if (<= (+ (Variables|Default|Gethp) (Variables|Default|GetCuracionBotiquin)) 1e+02)
      (Variables|Default|Sethp (+ (Variables|Default|Gethp) (Variables|Default|GetCuracionBotiquin)))
      (Variables|Default|SetBotiquin (- (Variables|Default|GetBotiquin) 1) :!label _label)
      (elif (== (Variables|Default|Gethp) 1e+02)
        (Development|PrintString "Tienes la vida al tope")
        (else
          (Variables|Default|Sethp 1e+02)
          (goto _label))))
    (else
      (Development|PrintString "Ups, no tenemos botiquines, consigue algunos para curarte"))))

(fn RecargarArma
  (if (> (Variables|Default|GetMunicionesActuales) 0)
    (if (> (Variables|Default|GetCargaMaximaCartucho) (Variables|Default|GetMunicionEnElCartucho))
      ;[1 1 1] Recargando
      (if (>= (Variables|Default|GetMunicionesActuales) (- (Variables|Default|GetCargaMaximaCartucho) (Variables|Default|GetMunicionEnElCartucho)))
        (Variables|Default|Setaux_recarga (- (Variables|Default|GetCargaMaximaCartucho) (Variables|Default|GetMunicionEnElCartucho)))
        (Variables|Default|SetMunicionEnElCartucho (+ (Variables|Default|GetMunicionEnElCartucho) (- (Variables|Default|GetCargaMaximaCartucho) (Variables|Default|GetMunicionEnElCartucho))))
        (Variables|Default|SetMunicionesActuales (- (Variables|Default|GetMunicionesActuales) (Variables|Default|Getaux_recarga)))
        (else
          (Variables|Default|SetMunicionEnElCartucho (+ (Variables|Default|GetMunicionEnElCartucho) (Variables|Default|GetMunicionesActuales)))
          (Variables|Default|SetMunicionesActuales 0))))
    (else
      (Development|PrintString "Consigue municiones"))))

(fn Shoot
  (if (> (Variables|Default|GetMunicionEnElCartucho) 0)
    (bind _result (Math|Integer|DecrementInt (Variables|Default|GetMunicionEnElCartucho))
      (:%20%20
        (Variables|Default|SetMunicionEnElCartucho _result)
        (return)))))